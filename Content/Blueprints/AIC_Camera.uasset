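; AI controller shared by security cameras and turrets that passes sight detections on to the pawn it possesses.
; On possess it caches the pawn as either a BP_SecurityCamera or a BP_Turret.
; Perception updates ignore actors tagged "AI", print the sensed actor and sense, and route sight stimuli to HandleSight.
; HandleSight forwards to the camera with the stimulus location, or to the turret without it.
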(event OnTargetPerceptionUpdated(AIPerception)
  (params (Actor :type Actor%20Object%20Reference) (Stimulus :type AI%20Stimulus%20Structure))
  (bind (_age _expirationage _strength _stimuluslocation _receiverlocation _tag _bsuccessfullysensed) (Utilities|Struct|BreakAIStimulus Stimulus))
  (if (not (Actor|ActorHasTag Actor "AI")) ; Ignore AI Actors
    (bind _returnvalue (Class|AIPerceptionSystem|GetSenseClassforStimulus Stimulus))
    (Development|PrintText (Utilities|Text|FormatText "Sensed: {actor} with {name}" Actor (Utilities|GetClassDisplayName _returnvalue)))
    (switch name _tag
      (:Default
        (switch string (Utilities|GetClassDisplayName _returnvalue)
          (:AISense_Sight
            (CallFunction|HandleSight Actor _bsuccessfullysensed _stimuluslocation)))))))

(event EventBeginPlay)

(event EventTick
  (params (DeltaSeconds :type Float%20%28single-precision%29)))

(event EventPossess
  (params (PossessedPawn :type Pawn%20Object%20Reference))
  (bind _asbp_security_camera (Utilities|Casting|CastToBP_SecurityCamera PossessedPawn)
    (:then
      (Variables|Default|SetAs%20BP%20Security%20Camera _asbp_security_camera))
    (:CastFailed
      (bind _asbp_turret (Utilities|Casting|CastToBP_Turret PossessedPawn))
      (Variables|Default|SetAs%20BP%20Turret _asbp_turret))))

(fn ConstructionScript)

(fn HandleSight
  (params (Target :type Actor%20Object%20Reference) (Successfully%20Sensed :type Boolean) (StimulusLocation :type Vector))
  (bind _as_bp_security_camera (Variables|Default|GetAs%20BP%20Security%20Camera)
    (:then
      (Default|HandleSight _as_bp_security_camera Target Successfully%20Sensed StimulusLocation))
    (:else
      (bind _as_bp_turret (Variables|Default|GetAs%20BP%20Turret)
        (:then
          (Default|HandleSight _as_bp_turret Target Successfully%20Sensed))
        (:else)))))