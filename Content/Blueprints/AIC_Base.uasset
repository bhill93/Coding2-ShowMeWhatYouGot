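; Base AI controller that turns perception updates into StateTree events, ignoring actors tagged as AI.
; Successful sight stores the sensed actor and sends an Attacking event, while lost sight only clears that actor.
; Both sight outcomes are forwarded to the possessed pawn through HandleSightMessage.
; Hearing, prediction and damage stimuli share one path that records the stimulus location as a point of interest and sends an Investigating event.
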(event OnTargetPerceptionUpdated(AIPerception)
  (params (Actor :type Actor%20Object%20Reference) (Stimulus :type AI%20Stimulus%20Structure))
  (bind (_age _expirationage _strength _stimuluslocation _receiverlocation _tag _bsuccessfullysensed) (Utilities|Struct|BreakAIStimulus Stimulus))
  (if (not (Actor|ActorHasTag Actor "AI"))
    (bind _returnvalue (Class|AIPerceptionSystem|GetSenseClassforStimulus Stimulus))
    (switch string (Utilities|GetClassDisplayName _returnvalue)
      (:AISense_Sight
        (if _bsuccessfullysensed
          (Variables|Default|SetSensedActor Actor)
          (Gameplay|StateTree|SendStateTreeEvent (Variables|Default|GetStateTreeAI) (Utilities|Struct|MakeStateTreeEvent "(TagName=\"AI.Event.Attacking\")") :!class /Script/GameplayStateTreeModule.StateTreeComponent)
          (else
            (Variables|Default|SetSensedActor 0)))
        (Class|BPIPerceiver|HandleSight(Message) (Variables|Default|GetPossessed%20Pawn) Actor _bsuccessfullysensed _stimuluslocation))
      (:AISense_Hearing
        (Variables|Default|SetPoint%20of%20Interest _stimuluslocation :!label _label)
        (Gameplay|StateTree|SendStateTreeEvent (Variables|Default|GetStateTreeAI) (Utilities|Struct|MakeStateTreeEvent "(TagName=\"AI.Event.Investigating\")") :!class /Script/GameplayStateTreeModule.StateTreeComponent))
      (:AISense_Prediction
        (goto _label))
      (:AISense_Damage
        (goto _label)))))

(event EventPossess
  (params (PossessedPawn :type Pawn%20Object%20Reference))
  (Variables|Default|SetPossessed%20Pawn PossessedPawn))

(fn ConstructionScript)