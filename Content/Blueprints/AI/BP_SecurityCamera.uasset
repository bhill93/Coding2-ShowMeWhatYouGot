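; BP_SecurityCamera is a security camera actor that raises an alarm when its AI Perception component sights a target.
; Perception updates are printed and filtered by sense class display name, with only sight passed to HandleSight.
; On sighting, it turns the camera material red, plays a sound and calls CheckOutSecurityAlarm on every BP_DumDum with a zero vector, not the stimulus location.
; Losing the target turns it green.
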(event OnTargetPerceptionUpdated(AIPerception)
  (params (Actor :type Actor%20Object%20Reference) (Stimulus :type AI%20Stimulus%20Structure))
  (bind (_age _expirationage _strength _stimuluslocation _receiverlocation _tag _bsuccessfullysensed) (Utilities|Struct|BreakAIStimulus Stimulus))
  (bind _returnvalue (Class|AIPerceptionSystem|GetSenseClassforStimulus Stimulus))
  (Development|PrintText (Utilities|Text|FormatText "Sensed: {actor} with {name}" (Utilities|GetClassDisplayName _returnvalue) Actor))
  (switch name _tag
    (:Default
      (switch string (Utilities|GetClassDisplayName _returnvalue)
        (:AISense_Sight
          (CallFunction|HandleSight Actor _bsuccessfullysensed _stimuluslocation))))))

(event OnTargetPerceptionForgotten(AIPerception)
  (params (Actor :type Actor%20Object%20Reference))
  (Development|PrintText (Utilities|Text|FormatText "Forgot about {actor}" Actor)))

(event OnTargetPerceptionInfoUpdated(AIPerception)
  (params (UpdateInfo :type Actor%20Perception%20Update%20Info%20Structure%20%28by%20ref%29)))

(event EventBeginPlay)

(event Collision|EventActorBeginOverlap
  (params (OtherActor :type Actor%20Object%20Reference)))

(event EventTick
  (params (DeltaSeconds :type Float%20%28single-precision%29)))

(fn ConstructionScript)

(fn HandleSight
  (params (Target :type Actor%20Object%20Reference) (Successfully%20Sensed :type Boolean) (StimulusLocation :type Vector))
  (bind _camera (Variables|Default|GetCamera))
  (if Successfully%20Sensed
    (Development|PrintText "Acquired Target")
    (Rendering|Material|SetMaterial _camera 0 "/AnimationSharing/AnimSharingRed.AnimSharingRed")
    (Audio|PlaySoundatLocation "/Engine/EditorSounds/Notifications/CompileFailed_Cue.CompileFailed_Cue" (Transformation|GetActorLocation) "0, 0, 0" 1.0 1.0 0.0 "/Game/Audio/NewAttenuation.NewAttenuation" 0 0 0)
    (bind _outactors (Actor|GetAllActorsOfClass "/Game/Blueprints/AI/BP_DumDum.BP_DumDum_C"))
    (for _array_element _outactors
      (Default|CheckOutSecurityAlarm _array_element "0, 0, 0"))
    (else
      (Development|PrintText "Lost Target")
      (Rendering|Material|SetMaterial _camera 0 "/AnimationSharing/AnimSharingGreen.AnimSharingGreen"))))