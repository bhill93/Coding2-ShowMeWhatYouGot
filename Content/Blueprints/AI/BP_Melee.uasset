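; BP_Melee is a melee AI pawn that tracks its own health and is controlled by an AIC_Base controller, cached on BeginPlay.
; Damage is reported to AI Damage sense and sent as a TookDamage event to the controller's State Tree, then subtracted from Health, destroying the actor at zero.
; DamageEnemy reuses the AnyDamage logic, and GetMedKit restores Health within a normalized 0–1 range.
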(event Custom|Get%20Med%20Kit
  (params (Health%20to%20Add :type Float%20%28double-precision%29))
  (Variables|Default|SetHealth (Math|Float|Clamp(Float) (+ (Variables|Default|GetHealth) Health%20to%20Add))))

(event Custom|DamageEnemy
  (Class|AISenseDamage|ReportDamageEvent self (stale Game|Damage|EventAnyDamage InstigatedBy) (stale Game|Damage|EventAnyDamage Damage) (Transformation|GetActorLocation (Pawn|GetControlledPawn (stale Game|Damage|EventAnyDamage InstigatedBy))) "0, 0, 0" "None")
  (Gameplay|StateTree|SendStateTreeEvent (Variables|/Game/Blueprints/AIC_Base.AIC_Base_C|GetStateTreeAI (Variables|Default|GetAs%20AIC%20Base)) (Utilities|Struct|MakeStateTreeEvent "(TagName=\"AI.Event.TookDamage\")") :!class /Script/GameplayStateTreeModule.StateTreeComponent)
  (bind _output_get (Variables|Default|SetHealth (- (Variables|Default|GetHealth) (stale Game|Damage|EventAnyDamage Damage))))
  (if (not (> _output_get 0.0))
    (Development|PrintText "We are DEAD")
    (Actor|DestroyActor) ; Replace with ragdoll
  ))

(event EventBeginPlay
  (bind _asaic_base (Utilities|Casting|CastToAIC_Base (Pawn|GetController)))
  (Variables|Default|SetAs%20AIC%20Base _asaic_base))

(event EventTick
  (params (DeltaSeconds :type Float%20%28single-precision%29)))

(event Game|Damage|EventAnyDamage
  (params (Damage :type Float%20%28single-precision%29) (DamageType :type Damage%20Type%20Object%20Reference) (InstigatedBy :type Controller%20Object%20Reference) (DamageCauser :type Actor%20Object%20Reference))
  (Class|AISenseDamage|ReportDamageEvent self InstigatedBy Damage (Transformation|GetActorLocation (Pawn|GetControlledPawn InstigatedBy)) "0, 0, 0" "None")
  (Gameplay|StateTree|SendStateTreeEvent (Variables|/Game/Blueprints/AIC_Base.AIC_Base_C|GetStateTreeAI (Variables|Default|GetAs%20AIC%20Base)) (Utilities|Struct|MakeStateTreeEvent "(TagName=\"AI.Event.TookDamage\")") :!class /Script/GameplayStateTreeModule.StateTreeComponent)
  (bind _output_get (Variables|Default|SetHealth (- (Variables|Default|GetHealth) Damage)))
  (if (not (> _output_get 0.0))
    (Development|PrintText "We are DEAD")
    (Actor|DestroyActor) ; Replace with ragdoll
  ))

(fn ConstructionScript)