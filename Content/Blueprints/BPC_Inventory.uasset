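; BPC_Inventory is an inventory component that stores items as an array of enum values indexed by slot.
; GetSlot resolves a slot's enum through GetItemDetails, which loops over every DT_Items row until one's Enum field matches.
; SetSlot writes one entry and calls OnSlotUpdated with its index, while Set Enum Array replaces the whole array and calls OnRefreshGrid.
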(event EventBeginPlay)

(event EventTick
  (params (DeltaSeconds :type Float%20%28single-precision%29)))

(fn GetItemDetails
  (params (RequestedItem :type E_Item%20Enum :default "NewEnumerator0"))
  (bind _outrownames (DataTable|GetDataTableRowNames "/Game/Blueprints/DataTables/DT_Items.DT_Items"))
  (for _array_element _outrownames ; Go through each row\nof the data table
    (bind _returnvalue (Utilities|GetDataTableRow "/Game/Blueprints/DataTables/DT_Items.DT_Items" _array_element)
      (:then
        (if (Utilities|Enum|Equal(Enum) (.Enum (Utilities|Struct|BreakS_Item _returnvalue)) RequestedItem) ; Did we find the enum we\nwere looking for?
          (return _returnvalue) ; Return the data table\nrow that was requested
        ))
      (:RowNotFound
        (Development|PrintString "RowNotFound")))))

(fn GetSlot
  (params (Requested%20Slot :type Integer))
  (bind _item_details (CallFunction|GetItemDetails (Utilities|Array|Get(acopy) (Variables|Default|GetEnumInventory) Requested%20Slot)))
  (return _item_details))

(fn SetSlot
  (params (Item :type E_Item%20Enum :default "NewEnumerator8") (Slot%20Index :type Integer))
  (Utilities|Array|SetArrayElem (Variables|Default|GetEnumInventory) Slot%20Index Item)
  (Default|CallOnSlotUpdated Slot%20Index))

(fn SetEnumArray
  (params (EnumInventory :type Array%20of%20E_Item%20Enums :default "NewEnumerator8"))
  (Variables|Default|SetEnumInventory EnumInventory)
  (Default|CallOnRefreshGrid))