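; BP_Chest is a chest actor that swings open when the first-person character enters its sphere and closes when they leave.
; A reversible timeline rotates the hinge, with a finished-opening branch that shows the chest menu and the player's inventory.
; That branch also registers the chest's inventory component with GM_SaveLoad's level state.
; LoadInventory replaces the component's contents with saved data.
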(event OnComponentBeginOverlap(Sphere)
  (params (OverlappedComponent :type Primitive%20Component%20Object%20Reference) (OtherActor :type Actor%20Object%20Reference) (OtherComp :type Primitive%20Component%20Object%20Reference) (OtherBodyIndex :type Integer) (bFromSweep :type Boolean) (SweepResult :type Hit%20Result%20Structure%20%28by%20ref%29))
  (bind _asbp_first_person_character (Utilities|Casting|CastToBP_FirstPersonCharacter OtherActor))
  (CallFunction|OpenChest false))

(event OnComponentEndOverlap(Sphere)
  (params (OverlappedComponent :type Primitive%20Component%20Object%20Reference) (OtherActor :type Actor%20Object%20Reference) (OtherComp :type Primitive%20Component%20Object%20Reference) (OtherBodyIndex :type Integer))
  (Utilities|Casting|CastToBP_FirstPersonCharacter OtherActor)
  (CallFunction|OpenChest true))

(event Custom|Open%20Chest
  (params (Reverse :type Boolean))
  (if Reverse
    (bind _newtrack_0 (Timeline|Open Reverse)
      (:Update
        (Transformation|SetRelativeRotation (Variables|Default|GetRealhinge) (Math|Rotator|MakeRotator (Math|Float|Lerp 0.0 -7e+01 _newtrack_0) 0.0 0.0) false false))
      (:Finished
        (if (not Reverse)
          (UserInterface|Viewport|AddtoViewport (Variables|Default|GetChestMenu) 0)
          (Default|OpenInventory (stale OnComponentBeginOverlap(Sphere) _asbp_first_person_character))
          (bind _asgm_save_load (Utilities|Casting|CastToGM_SaveLoad (Game|GetGameMode)))
          (Default|AddInventory (Variables|/Game/Blueprints/SaveLoad/GM_SaveLoad.GM_SaveLoad_C|GetLevelState _asgm_save_load) (Variables|Default|GetBPC_Inventory)))))
    (else
      (Timeline|Open Play))))

(event Custom|Load%20Inventory
  (params (EnumInventory :type Array%20of%20E_Item%20Enums :default "NewEnumerator8"))
  (Variables|/Game/Blueprints/BPC_Inventory.BPC_Inventory_C|SetEnumInventory (Variables|Default|GetBPC_Inventory) EnumInventory) ; Replace Inventory with\nsaved Inventory
)

(event EventBeginPlay
  (bind _returnvalue (UserInterface|CreateWidget "/Game/Widgets/W_ChestMenu.W_ChestMenu_C" 0 (Variables|Default|GetBPC_Inventory))) ; Create now, show later
  (Variables|Default|SetChestMenu _returnvalue))

(fn ConstructionScript)