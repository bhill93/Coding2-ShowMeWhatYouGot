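; Key pickup actor that the first-person player can collect from within its trigger volume.
; Entering the trigger creates a new Press E widget and registers the key on BP_FirstPersonCharacter; leaving hides the prompt and clears that reference.
; The Pickup event prints a found message and destroys the actor, while Drop, Use and AlternateUse are empty.
; PlayerInRange is set before the character cast, so any overlapping actor toggles it.
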(event OnComponentBeginOverlap(Trigger)
  (params (OverlappedComponent :type Primitive%20Component%20Object%20Reference) (OtherActor :type Actor%20Object%20Reference) (OtherComp :type Primitive%20Component%20Object%20Reference) (OtherBodyIndex :type Integer) (bFromSweep :type Boolean) (SweepResult :type Hit%20Result%20Structure%20%28by%20ref%29))
  (Variables|Default|SetPlayerInRange true)
  (bind _asbp_first_person_character (Utilities|Casting|CastToBP_FirstPersonCharacter OtherActor))
  (bind _returnvalue (UserInterface|CreateWidget "/Game/Widgets/W_PressE.W_PressE_C"))
  (UserInterface|Viewport|AddtoViewport _returnvalue 0)
  (Widget|SetVisibility _returnvalue "Visible")
  (Variables|/Game/FirstPerson/Blueprints/BP_FirstPersonCharacter.BP_FirstPersonCharacter_C|SetKey _asbp_first_person_character self))

(event OnComponentEndOverlap(Trigger)
  (params (OverlappedComponent :type Primitive%20Component%20Object%20Reference) (OtherActor :type Actor%20Object%20Reference) (OtherComp :type Primitive%20Component%20Object%20Reference) (OtherBodyIndex :type Integer))
  (Variables|Default|SetPlayerInRange false)
  (bind _asbp_first_person_character (Utilities|Casting|CastToBP_FirstPersonCharacter OtherActor))
  (Widget|SetVisibility (stale OnComponentBeginOverlap(Trigger) _returnvalue) "Hidden")
  (Variables|/Game/FirstPerson/Blueprints/BP_FirstPersonCharacter.BP_FirstPersonCharacter_C|SetKey _asbp_first_person_character 0))

(event EventBeginPlay
  (Input|EnableInput (Game|GetPlayerController 0) 0))

(event Collision|EventActorBeginOverlap
  (params (OtherActor :type Actor%20Object%20Reference)))

(event EventTick
  (params (DeltaSeconds :type Float%20%28single-precision%29)))

(event EventPickup
  (Development|PrintText "You found a key!")
  (Actor|DestroyActor))

(event EventAlternateUse)

(event EventUse)

(event EventDrop)

(fn ConstructionScript)