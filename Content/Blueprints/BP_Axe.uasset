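; Axe item that the first-person player can pick up, swing, throw or drop.
; Trigger overlap shows a press-E widget and registers the axe on the character; leaving hides it but clears Gun, not Axe.
; Pickup disables Box collision, while Drop restores physics and applies a forward impulse.
; Use swings the mesh via a pitch timeline; AlternateUse launches Pistol001Obj with physics and an impulse, starting a rotation timeline.
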(event OnComponentBeginOverlap(Trigger)
  (params (OverlappedComponent :type Primitive%20Component%20Object%20Reference) (OtherActor :type Actor%20Object%20Reference) (OtherComp :type Primitive%20Component%20Object%20Reference) (OtherBodyIndex :type Integer) (bFromSweep :type Boolean) (SweepResult :type Hit%20Result%20Structure%20%28by%20ref%29))
  (Variables|Default|SetcanPickUpFirearm true)
  (bind _asbp_first_person_character (Utilities|Casting|CastToBP_FirstPersonCharacter OtherActor))
  (bind _returnvalue (UserInterface|CreateWidget "/Game/Widgets/W_PressE.W_PressE_C"))
  (UserInterface|Viewport|AddtoViewport _returnvalue 0)
  (Widget|SetVisibility _returnvalue "Visible")
  (Variables|/Game/FirstPerson/Blueprints/BP_FirstPersonCharacter.BP_FirstPersonCharacter_C|SetAxe _asbp_first_person_character self))

(event OnComponentEndOverlap(Trigger)
  (params (OverlappedComponent :type Primitive%20Component%20Object%20Reference) (OtherActor :type Actor%20Object%20Reference) (OtherComp :type Primitive%20Component%20Object%20Reference) (OtherBodyIndex :type Integer))
  (Variables|Default|SetcanPickUpFirearm false)
  (bind _asbp_first_person_character (Utilities|Casting|CastToBP_FirstPersonCharacter OtherActor))
  (Widget|SetVisibility (stale OnComponentBeginOverlap(Trigger) _returnvalue) "Hidden")
  (Variables|/Game/FirstPerson/Blueprints/BP_FirstPersonCharacter.BP_FirstPersonCharacter_C|SetGun _asbp_first_person_character 0))

(event Custom|SwingAxe
  (params (Reverse :type Boolean))
  (if Reverse
    (bind _newtrack_0 (Timeline|Timeline Reverse)
      (:Update
        (Transformation|SetRelativeRotation (Variables|Default|GetStaticMesh) (Math|Rotator|MakeRotator 0.0 (Math|Float|Lerp 0.0 -9e+01 _newtrack_0) 0.0) false false)))
    (else
      (Timeline|Timeline PlayFromStart))))

(event Custom|ThrowAxe
  (params (Stop :type Boolean))
  (bind _pistol_001_obj (Variables|Default|Getpistol_001_obj))
  (Collision|SetCollisionEnabled _pistol_001_obj "QueryAndPhysics")
  (Physics|SetSimulatePhysics _pistol_001_obj true)
  (Transformation|SetRelativeRotation (Variables|Default|GetStaticMesh) (Math|Rotator|MakeRotator 0.0 (Math|Float|Lerp 0.0 -1.8e+02 (stale _newtrack_0)) 0.0) false false)
  (Physics|AddImpulse _pistol_001_obj (* (Math|Vector|GetForwardVector (Variables|Default|GetStaticMesh)) 3e+03) "None" false)
  (bind _newtrack_0 (Timeline|AxeRotation PlayFromStart)))

(event EventBeginPlay
  (bind _returnvalue (Actor|GetActorOfClass "/Game/FirstPerson/Blueprints/BP_FirstPersonCameraManager.BP_FirstPersonCameraManager_C"))
  (Variables|Default|SetCamera _returnvalue))

(event Collision|EventActorBeginOverlap
  (params (OtherActor :type Actor%20Object%20Reference)))

(event EventTick
  (params (DeltaSeconds :type Float%20%28single-precision%29)))

(event EventPickup
  (params (Owner :type BPC%20Interact%20Object%20Reference))
  (Development|PrintText "You have an axe")
  (Collision|SetCollisionEnabled (Variables|Default|GetBox) "NoCollision"))

(event EventAlternateUse
  (CallFunction|ThrowAxe false))

(event EventUse
  (CallFunction|SwingAxe false))

(event EventDrop
  (bind _box (Variables|Default|GetBox))
  (Variables|/Game/Blueprints/BPC_Interact.BPC_Interact_C|SetHeldItem (stale EventPickup Owner) 0)
  (Collision|SetCollisionEnabled _box "QueryAndPhysics")
  (Physics|SetSimulatePhysics _box true)
  (Physics|AddImpulse _box (* (Math|Vector|GetForwardVector _box) 1e+03) "None" false))

(fn ConstructionScript)