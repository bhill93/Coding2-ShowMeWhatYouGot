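; BP_Checkpoint is a checkpoint actor that saves the player's progress when the first-person character overlaps it.
; On BeginPlay it caches the GM_SaveLoad game mode.
; On overlap it passes the character's belt and backpack inventory enums and current transform to the game mode's Save function, then prints a confirmation message.
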(event EventBeginPlay
  (bind _asgm_save_load (Utilities|Casting|CastToGM_SaveLoad (Game|GetGameMode)))
  (Variables|Default|SetGameMode _asgm_save_load))

(event Collision|EventActorBeginOverlap
  (params (OtherActor :type Actor%20Object%20Reference))
  (bind _asbp_first_person_character (Utilities|Casting|CastToBP_FirstPersonCharacter OtherActor)) ; When player overlaps, call the save function\non the Game Mode
  (Default|Save (Variables|Default|GetGameMode) (Variables|/Game/Blueprints/BPC_Inventory.BPC_Inventory_C|GetEnumInventory (Variables|/Game/FirstPerson/Blueprints/BP_FirstPersonCharacter.BP_FirstPersonCharacter_C|GetBPC_BeltInv _asbp_first_person_character)) (Variables|/Game/Blueprints/BPC_Inventory.BPC_Inventory_C|GetEnumInventory (Variables|/Game/FirstPerson/Blueprints/BP_FirstPersonCharacter.BP_FirstPersonCharacter_C|GetBPC_BackpackInv _asbp_first_person_character)) (Transformation|GetActorTransform _asbp_first_person_character))
  (Development|PrintString "Checkpoint activated"))

(event EventTick
  (params (DeltaSeconds :type Float%20%28single-precision%29)))

(fn ConstructionScript)