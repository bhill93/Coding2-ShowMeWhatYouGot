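; Game mode that saves and restores player inventory and per-level state through two save game slots.
; BeginPlay creates SG_Player and SG_LevelState objects when missing, or calls Load for existing saves, briefly delayed for the player's.
; Save writes belt and backpack to the player slot, and player transform to a slot named after the level.
; Load reads both slots, refills BP_FirstPersonCharacter's inventories, activates saved actors and restores its transform.
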(event EventBeginPlay
  (Development|PrintText "Starting GM_SaveLoad" true true "(R=0.000000,G=0.660000,B=1.000000,A=1.000000)" 5.0)
  (Utilities|FlowControl|Sequence
    (:then_0
      (bind _returnvalue (SaveGame|DoesSaveGameExist (Variables|Default|GetSlot%20Name)))
      (if _returnvalue
        (Utilities|FlowControl|Delay 0.2)
        (CallFunction|Load)
        (Development|PrintString "LoadedGame")
        (else
          (bind _returnvalue_2 (SaveGame|CreateSaveGameObject "/Game/Blueprints/SaveLoad/SG_Player.SG_Player_C"))
          (Variables|Default|SetPlayerSave _returnvalue_2))))
    (:then_1
      ;[0.15 0.15 0.15 0.5] Load or create level state save
      (bind _returnvalue_3 (Game|GetCurrentLevelName true))
      (bind _returnvalue_4 (SaveGame|DoesSaveGameExist _returnvalue_3))
      (if _returnvalue_4
        (CallFunction|Load)
        (else
          (bind _returnvalue_5 (SaveGame|CreateSaveGameObject "/Game/Blueprints/SaveLoad/SG_LevelState.SG_LevelState_C"))
          (Variables|Default|SetLevelState _returnvalue_5))))))

(event EventTick
  (params (DeltaSeconds :type Float%20%28single-precision%29)))

(fn ConstructionScript)

(fn Save
  (params (Belt :type Array%20of%20E_Item%20Enums :default "NewEnumerator8") (PlayerInv :type Array%20of%20E_Item%20Enums :default "NewEnumerator8") (InputPin :type Transform))
  (bind _playersave (Variables|Default|GetPlayerSave))
  (Utilities|FlowControl|Sequence
    (:then_0
      ;[0.15 0.15 0.15 0.5] Save Player Stats
      (Variables|/Game/Blueprints/SaveLoad/SG_Player.SG_Player_C|SetBelt _playersave Belt)
      (Variables|/Game/Blueprints/SaveLoad/SG_Player.SG_Player_C|SetPlayerInv _playersave PlayerInv)
      (SaveGame|SaveGametoSlot (Variables|Default|GetPlayerSave) (Variables|Default|GetSlot%20Name)) ; Save game to file (Player
    )
    (:then_1
      (Variables|/Game/Blueprints/SaveLoad/SG_LevelState.SG_LevelState_C|SetPlayerTransf (Variables|Default|GetLevelState) InputPin)
      ;[0.15 0.15 0.15 0.5] Save Level State
      (bind _returnvalue (Game|GetCurrentLevelName true))
      (SaveGame|SaveGametoSlot (Variables|Default|GetLevelState) _returnvalue) ; Save Level state
    )))

(fn Load
  (Utilities|FlowControl|Sequence
    (:then_0
      (bind _returnvalue (SaveGame|LoadGamefromSlot (Variables|Default|GetSlot%20Name))) ; Load from file
      (bind _assg_player (Utilities|Casting|CastToSG_Player _returnvalue)) ; Cast to specific SG_Player
      (Variables|Default|SetPlayerSave _assg_player) ; Store player save
      (bind _asbp_first_person_character (Utilities|Casting|CastToBP_FirstPersonCharacter (Game|GetPlayerCharacter 0))) ; Get reference to Player
      (Default|SetEnumArray (Variables|/Game/FirstPerson/Blueprints/BP_FirstPersonCharacter.BP_FirstPersonCharacter_C|GetBPC_BeltInv _asbp_first_person_character) (Variables|/Game/Blueprints/SaveLoad/SG_Player.SG_Player_C|GetBelt (Variables|Default|GetPlayerSave)))
      (Default|SetEnumArray (Variables|/Game/FirstPerson/Blueprints/BP_FirstPersonCharacter.BP_FirstPersonCharacter_C|GetBPC_BackpackInv _asbp_first_person_character) (Variables|/Game/Blueprints/SaveLoad/SG_Player.SG_Player_C|GetPlayerInv (Variables|Default|GetPlayerSave)))
      (Development|PrintText "Inventory Updated"))
    (:then_1
      (bind _returnvalue_2 (Game|GetCurrentLevelName true))
      (bind _returnvalue_3 (SaveGame|LoadGamefromSlot _returnvalue_2))
      (bind _assg_level_state (Utilities|Casting|CastToSG_LevelState _returnvalue_3))
      (bind _output_get (Variables|Default|SetLevelState _assg_level_state))
      (Default|ActivateActors _output_get)
      (bind _asbp_first_person_character_2 (Utilities|Casting|CastToBP_FirstPersonCharacter (Game|GetPlayerCharacter 0))) ; Get reference to Player
      (Default|LoadTransform _asbp_first_person_character_2 (Variables|/Game/Blueprints/SaveLoad/SG_LevelState.SG_LevelState_C|GetPlayerTransf (Variables|Default|GetLevelState))))))