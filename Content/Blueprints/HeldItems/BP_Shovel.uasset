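; Held shovel item that the player can pick up and throw when dropped.
; Pickup turns off collision on the box and both shovel meshes and returns the Item value.
; Drop restores collision, enables physics on the box and launches it along its forward vector with a mass-independent impulse.
; BeginPlay enables input for the first player controller, while Use and AlternateUse are empty stubs.
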(event EventBeginPlay
  (Input|EnableInput (Game|GetPlayerController 0) 0))

(event Collision|EventActorBeginOverlap
  (params (OtherActor :type Actor%20Object%20Reference)))

(event EventAlternateUse)

(event EventUse)

(event EventDrop
  (bind _boxcollision (Variables|Default|GetBoxCollision))
  (Collision|SetCollisionEnabled _boxcollision "QueryAndPhysics")
  (Physics|SetSimulatePhysics _boxcollision true)
  (Physics|AddImpulse _boxcollision (* (Math|Vector|GetForwardVector _boxcollision) 1e+03) "None" true) ; Throw object forward
)

(fn ConstructionScript)

(fn Pickup
  (params (Owner :type BPC%20Interact%20Object%20Reference))
  (Collision|SetCollisionEnabled (Variables|Default|GetBoxCollision) "NoCollision")
  (return (Variables|Default|GetItem)))