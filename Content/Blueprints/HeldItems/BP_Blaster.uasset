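; Held blaster pistol that the player can pick up, drop, fire and aim down sights.
; Pickup stores the owner and disables box collision; Drop clears the held item and throws the gun with physics.
; Use launches a physics bullet from the muzzle, enabling its collision after a short delay.
; AlternateUse toggles aiming, with timelines setting fixed camera FOVs and offsetting the mesh on aim-in, while the aim-out offsets are unwired.
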(event Custom|AimDownSights
  (Variables|Default|SetisAiming true)
  (Timeline|FIeldOfView Play
    (:Update
      (Camera|SetFieldOfView (Variables|Default|GetPlayerCam) 5e+01)
      (if (Variables|Default|GetisAiming)
        (bind _newtrack_0 (Timeline|MoveGun PlayFromStart)
          (:Update
            (Transformation|AddLocalOffset (Variables|Default|Getpistol_001_obj) (Math|Vector|MakeVector (Math|Float|Lerp 0.0 1.0 _newtrack_0) (Math|Float|Lerp 0.0 1.0 _newtrack_0) (Math|Float|Lerp 0.0 1.0 _newtrack_0)) false false)))
        (else
          (Timeline|MoveGun Reverse))))))

(event Custom|StopAiming
  (Variables|Default|SetisAiming false)
  (Timeline|Timeline PlayFromStart
    (:Update
      (Camera|SetFieldOfView (Variables|Default|GetPlayerCam) 1e+02)
      (bind _newtrack_0 (Timeline|Timeline_0 PlayFromStart)))))

(event EventBeginPlay
  (bind _returnvalue (Actor|GetActorOfClass "/Game/FirstPerson/Blueprints/BP_FirstPersonCameraManager.BP_FirstPersonCameraManager_C"))
  (Variables|Default|SetCamera _returnvalue)
  (bind _returnvalue_2 (Actor|GetActorOfClass "/Game/FirstPerson/Blueprints/BP_FirstPersonCharacter.BP_FirstPersonCharacter_C"))
  (Variables|Default|SetPlayerCam (Variables|/Game/FirstPerson/Blueprints/BP_FirstPersonCharacter.BP_FirstPersonCharacter_C|GetFirstPersonCamera _returnvalue_2)))

(event Collision|EventActorBeginOverlap
  (params (OtherActor :type Actor%20Object%20Reference)))

(event EventTick
  (params (DeltaSeconds :type Float%20%28single-precision%29)))

(event EventAlternateUse
  (if (Variables|Default|GetisAiming)
    (CallFunction|StopAiming)
    (else
      (CallFunction|AimDownSights))))

(event EventUse
  (bind _muzzlelocation (Variables|Default|GetMuzzleLocation))
  (bind _returnvalue (Game|SpawnActorfromClass "/Game/Blueprints/HeldItems/BP_Bullet.BP_Bullet_C" (Transformation|GetWorldTransform _muzzlelocation) "AlwaysSpawn" "MultiplyWithRoot" 0 0))
  (Physics|SetSimulatePhysics (Variables|/Game/Blueprints/HeldItems/BP_Bullet.BP_Bullet_C|GetBullet _returnvalue) true)
  (Physics|AddImpulse (Variables|/Game/Blueprints/HeldItems/BP_Bullet.BP_Bullet_C|GetBullet _returnvalue) (* (Math|Vector|GetForwardVector _muzzlelocation) 2.5e+03) "None" true)
  (Utilities|FlowControl|Delay 0.2)
  (Collision|SetCollisionEnabled (Variables|/Game/Blueprints/HeldItems/BP_Bullet.BP_Bullet_C|GetBullet _returnvalue) "QueryAndPhysics"))

(event EventDrop
  (bind _box (Variables|Default|GetBox))
  (Variables|/Game/Blueprints/BPC_Interact.BPC_Interact_C|SetHeldItem (Variables|Default|GetOwnerr) 0)
  (Collision|SetCollisionEnabled _box "QueryAndPhysics")
  (Physics|SetSimulatePhysics _box true)
  (Physics|AddImpulse _box (* (Math|Vector|GetForwardVector _box) 1e+03) "None" false))

(fn ConstructionScript)

(fn Pickup
  (params (Owner :type BPC%20Interact%20Object%20Reference))
  (Variables|Default|SetOwnerr Owner)
  (Collision|SetCollisionEnabled (Variables|Default|GetBox) "NoCollision")
  (return (Variables|Default|GetItem%20Type)))