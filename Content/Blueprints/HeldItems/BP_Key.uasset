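; BP_Key is a held key item that the player picks up, throws or uses to open a BP_Door.
; Its trigger shows a press-E widget and registers the key on the first-person character while in range.
; Pickup stores the owner, disables collision and adds the key to the save/load level state.
; Drop re-enables physics with a forward impulse, while Use line-traces ahead, opens a hit door and destroys the key.
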(event OnComponentBeginOverlap(Trigger)
  (params (OverlappedComponent :type Primitive%20Component%20Object%20Reference) (OtherActor :type Actor%20Object%20Reference) (OtherComp :type Primitive%20Component%20Object%20Reference) (OtherBodyIndex :type Integer) (bFromSweep :type Boolean) (SweepResult :type Hit%20Result%20Structure%20%28by%20ref%29))
  (Variables|Default|SetPlayerInRange true)
  (bind _asbp_first_person_character (Utilities|Casting|CastToBP_FirstPersonCharacter OtherActor))
  (bind _returnvalue (UserInterface|CreateWidget "/Game/Widgets/W_PressE.W_PressE_C"))
  (UserInterface|Viewport|AddtoViewport _returnvalue 0)
  (Widget|SetVisibility _returnvalue "Visible")
  (Variables|/Game/FirstPerson/Blueprints/BP_FirstPersonCharacter.BP_FirstPersonCharacter_C|SetKey _asbp_first_person_character self))

(event OnComponentEndOverlap(Trigger)
  (params (OverlappedComponent :type Primitive%20Component%20Object%20Reference) (OtherActor :type Actor%20Object%20Reference) (OtherComp :type Primitive%20Component%20Object%20Reference) (OtherBodyIndex :type Integer))
  (Variables|Default|SetPlayerInRange false)
  (bind _asbp_first_person_character (Utilities|Casting|CastToBP_FirstPersonCharacter OtherActor))
  (Widget|SetVisibility (stale OnComponentBeginOverlap(Trigger) _returnvalue) "Hidden")
  (Variables|/Game/FirstPerson/Blueprints/BP_FirstPersonCharacter.BP_FirstPersonCharacter_C|SetKey _asbp_first_person_character 0))

(event EventBeginPlay
  (Input|EnableInput (Game|GetPlayerController 0) 0))

(event Collision|EventActorBeginOverlap
  (params (OtherActor :type Actor%20Object%20Reference)))

(event EventTick
  (params (DeltaSeconds :type Float%20%28single-precision%29)))

(event EventAlternateUse)

(event EventUse
  (bind _boxcollision (Variables|Default|GetBoxCollision))
  (bind _returnvalue (Transformation|GetWorldLocation _boxcollision))
  (bind _outhit (Collision|LineTraceByChannel _returnvalue (+ _returnvalue (* (Math|Vector|GetForwardVector _boxcollision) 3e+02)) "TraceTypeQuery1" false 0 "ForDuration"))
  (bind _asbp_door (Utilities|Casting|CastToBP_Door (.HitActor (Collision|BreakHitResult _outhit))))
  (Default|OpenDoor _asbp_door)
  (Variables|/Game/Blueprints/BPC_Interact.BPC_Interact_C|SetHeldItem (Variables|Default|GetOwnerr) 0) ; Set "held item" to nothing
  (Actor|DestroyActor self))

(event EventDrop
  (bind _boxcollision (Variables|Default|GetBoxCollision))
  (Variables|/Game/Blueprints/BPC_Interact.BPC_Interact_C|SetHeldItem (Variables|Default|GetOwnerr) 0) ; Set "held item" to nothing
  (Collision|SetCollisionEnabled _boxcollision "QueryAndPhysics")
  (Physics|SetSimulatePhysics _boxcollision true)
  (Physics|AddImpulse _boxcollision (* (Math|Vector|GetForwardVector _boxcollision) 1e+03) "None" true) ; Throw object forward
)

(fn ConstructionScript)

(fn Pickup
  (params (Owner :type BPC%20Interact%20Object%20Reference))
  (Variables|Default|SetOwnerr Owner)
  (Collision|SetCollisionEnabled (Variables|Default|GetBoxCollision) "NoCollision")
  ;[0.15 0.15 0.15 0.5] Already picked up so do not load into level
  (bind _asgm_save_load (Utilities|Casting|CastToGM_SaveLoad (Game|GetGameMode)))
  (Default|AddActors (Variables|/Game/Blueprints/SaveLoad/GM_SaveLoad.GM_SaveLoad_C|GetLevelState _asgm_save_load) self)
  (return (Variables|Default|GetItem)))