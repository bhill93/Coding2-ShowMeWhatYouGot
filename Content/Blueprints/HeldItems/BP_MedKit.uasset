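; Med kit pickup that calls GetMedKit on a BP_Melee or first-person character overlapping its cube, then destroys itself.
; It also works as a held item: Pickup stores the owner and disables collision, while Drop restores physics and throws it forward.
; Use line-traces ahead and, on hitting a BP_Door, opens it and consumes the item, logic that involves no healing.
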(event OnComponentBeginOverlap(Cube)
  (params (OverlappedComponent :type Primitive%20Component%20Object%20Reference) (OtherActor :type Actor%20Object%20Reference) (OtherComp :type Primitive%20Component%20Object%20Reference) (OtherBodyIndex :type Integer) (bFromSweep :type Boolean) (SweepResult :type Hit%20Result%20Structure%20%28by%20ref%29))
  (bind _asbp_melee (Utilities|Casting|CastToBP_Melee OtherActor)
    (:then
      (Default|GetMedKit _asbp_melee 0.25))
    (:CastFailed
      (bind _asbp_first_person_character (Utilities|Casting|CastToBP_FirstPersonCharacter OtherActor))
      (Default|GetMedKit _asbp_first_person_character 0.25)))
  (Development|PrintString "I HAVE BEEN PICKED UP" true true "(R=0.000000,G=0.000000,B=0.000000,A=1.000000)" 4.0)
  (Actor|DestroyActor))

(event EventBeginPlay
  (Input|EnableInput (Game|GetPlayerController 0) 0))

(event Collision|EventActorBeginOverlap
  (params (OtherActor :type Actor%20Object%20Reference)))

(event EventTick
  (params (DeltaSeconds :type Float%20%28single-precision%29)))

(event EventAlternateUse)

(event EventUse
  (bind _cube (Variables|Default|GetCube))
  (bind _returnvalue (Transformation|GetWorldLocation _cube))
  (bind _outhit (Collision|LineTraceByChannel _returnvalue (+ _returnvalue (* (Math|Vector|GetForwardVector _cube) 3e+02)) "TraceTypeQuery1" false 0 "ForDuration"))
  (bind _asbp_door (Utilities|Casting|CastToBP_Door (.HitActor (Collision|BreakHitResult _outhit))))
  (Default|OpenDoor _asbp_door)
  (Variables|/Game/Blueprints/BPC_Interact.BPC_Interact_C|SetHeldItem (Variables|Default|GetOwnerr) 0) ; Set "held item" to nothing
  (Actor|DestroyActor self))

(event EventDrop
  (bind _cube (Variables|Default|GetCube))
  (Variables|/Game/Blueprints/BPC_Interact.BPC_Interact_C|SetHeldItem (Variables|Default|GetOwnerr) 0) ; Set "held item" to nothing
  (Collision|SetCollisionEnabled _cube "QueryAndPhysics")
  (Physics|SetSimulatePhysics _cube true)
  (Physics|AddImpulse _cube (* (Math|Vector|GetForwardVector _cube) 1e+03) "None" true) ; Throw object forward
)

(fn ConstructionScript)

(fn Pickup
  (params (Owner :type BPC%20Interact%20Object%20Reference))
  (Variables|Default|SetOwnerr Owner)
  (Collision|SetCollisionEnabled (Variables|Default|GetCube) "NoCollision")
  (return (Variables|Default|GetItem)))