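; BP_Axe is a held axe item with pickup, drop, a primary swing and an alternate chop.
; Pickup stores the owner and disables collision; Drop clears the owner's HeldItem, enables physics on Pistol001Obj and flings it along its forward vector.
; Use and AlternateUse play separate timelines that lerp that component's relative rotation, yaw for the attack and pitch for the chop.
; The swings only animate, with no hit or damage logic.
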(event Custom|ChopAxe
  (params (Reverse :type Boolean))
  (if Reverse
    (bind _newtrack_0 (Timeline|Timeline Reverse)
      (:Update
        (Transformation|SetRelativeRotation (Variables|Default|Getpistol_001_obj) (Math|Rotator|MakeRotator 0.0 (Math|Float|Lerp 0.0 -9e+01 _newtrack_0) 0.0) false false)))
    (else
      (Timeline|Timeline PlayFromStart))))

(event Custom|AxeAttack
  (params (Reverse :type Boolean))
  (if Reverse
    (bind _newtrack_0 (Timeline|Timeline_0 Reverse)
      (:Update
        (Transformation|SetRelativeRotation (Variables|Default|Getpistol_001_obj) (Math|Rotator|MakeRotator 9e+01 0.0 (Math|Float|Lerp 0.0 -1.5e+02 _newtrack_0)) false false)))
    (else
      (Timeline|Timeline_0 PlayFromStart))))

(event EventBeginPlay
  (bind _returnvalue (Actor|GetActorOfClass "/Game/FirstPerson/Blueprints/BP_FirstPersonCameraManager.BP_FirstPersonCameraManager_C"))
  (Variables|Default|SetCamera _returnvalue))

(event Collision|EventActorBeginOverlap
  (params (OtherActor :type Actor%20Object%20Reference)))

(event EventTick
  (params (DeltaSeconds :type Float%20%28single-precision%29)))

(event EventAlternateUse
  (CallFunction|ChopAxe false))

(event EventUse
  (CallFunction|AxeAttack false))

(event EventDrop
  (bind _pistol_001_obj (Variables|Default|Getpistol_001_obj))
  (Variables|/Game/Blueprints/BPC_Interact.BPC_Interact_C|SetHeldItem (Variables|Default|GetOwnerr) 0)
  (Collision|SetCollisionEnabled _pistol_001_obj "QueryAndPhysics")
  (Physics|SetSimulatePhysics _pistol_001_obj true)
  (Physics|AddImpulse _pistol_001_obj (* (Math|Vector|GetForwardVector _pistol_001_obj) 1e+03) "None" true))

(fn ConstructionScript)

(fn Pickup
  (params (Owner :type BPC%20Interact%20Object%20Reference))
  (Variables|Default|SetOwnerr Owner)
  (Collision|SetCollisionEnabled (Variables|Default|GetBox) "NoCollision")
  (return (Variables|Default|GetItem)))