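; BP_Hammer is a held item that opens a BP_Door and is consumed in the process.
; Pickup stores the owner, disables collision and returns the item.
; Use line-traces forward from the box collision with debug drawing, and on a door hit calls OpenDoor, clears the owner's held item and destroys the hammer.
; Drop clears the held item, restores collision and physics, and throws the hammer forward with an impulse.
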(event EventBeginPlay
  (Input|EnableInput (Game|GetPlayerController 0) 0))

(event Collision|EventActorBeginOverlap
  (params (OtherActor :type Actor%20Object%20Reference)))

(event EventAlternateUse)

(event EventUse
  (bind _boxcollision (Variables|Default|GetBoxCollision))
  (bind _returnvalue (Transformation|GetWorldLocation _boxcollision))
  (bind _outhit (Collision|LineTraceByChannel _returnvalue (+ _returnvalue (* (Math|Vector|GetForwardVector _boxcollision) 3e+02)) "TraceTypeQuery1" false 0 "ForDuration"))
  (bind _asbp_door (Utilities|Casting|CastToBP_Door (.HitActor (Collision|BreakHitResult _outhit))))
  (Default|OpenDoor _asbp_door)
  (Variables|/Game/Blueprints/BPC_Interact.BPC_Interact_C|SetHeldItem (Variables|Default|GetOwnerr) 0) ; Set "held item" to nothing
  (Actor|DestroyActor self))

(event EventDrop
  (bind _boxcollision (Variables|Default|GetBoxCollision))
  (Variables|/Game/Blueprints/BPC_Interact.BPC_Interact_C|SetHeldItem (Variables|Default|GetOwnerr) 0) ; Set "held item" to nothing
  (Collision|SetCollisionEnabled _boxcollision "QueryAndPhysics")
  (Physics|SetSimulatePhysics _boxcollision true)
  (Physics|AddImpulse _boxcollision (* (Math|Vector|GetForwardVector _boxcollision) 1e+03) "None" true) ; Throw object forward
)

(fn ConstructionScript)

(fn Pickup
  (params (Owner :type BPC%20Interact%20Object%20Reference))
  (Variables|Default|SetOwnerr Owner)
  (Collision|SetCollisionEnabled (Variables|Default|GetBoxCollision) "NoCollision")
  (return (Variables|Default|GetItem)))