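; BP_Door is an interactive cabin door that opens by rotating the whole actor 90 degrees in yaw.
; Overlapping its collider while closed shows the W_PressE prompt and registers the door on the first-person character; leaving clears both.
; Activation adds the door to the GM_SaveLoad game mode's LevelState before rotating it.
; The construction script applies a configurable DoorRotation yaw to the mesh.
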(event OnComponentBeginOverlap(Collider)
  (params (OverlappedComponent :type Primitive%20Component%20Object%20Reference) (OtherActor :type Actor%20Object%20Reference) (OtherComp :type Primitive%20Component%20Object%20Reference) (OtherBodyIndex :type Integer) (bFromSweep :type Boolean) (SweepResult :type Hit%20Result%20Structure%20%28by%20ref%29))
  (if (not (Variables|Default|GetdoorIsOpen))
    (Variables|Default|SetcanOpenDoor true)
    (bind _asbp_first_person_character (Utilities|Casting|CastToBP_FirstPersonCharacter OtherActor))
    (bind _returnvalue (UserInterface|CreateWidget "/Game/Widgets/W_PressE.W_PressE_C"))
    (UserInterface|Viewport|AddtoViewport _returnvalue 0)
    (Widget|SetVisibility _returnvalue "Visible")
    (Variables|/Game/FirstPerson/Blueprints/BP_FirstPersonCharacter.BP_FirstPersonCharacter_C|SetDoor _asbp_first_person_character self)))

(event OnComponentEndOverlap(Collider)
  (params (OverlappedComponent :type Primitive%20Component%20Object%20Reference) (OtherActor :type Actor%20Object%20Reference) (OtherComp :type Primitive%20Component%20Object%20Reference) (OtherBodyIndex :type Integer))
  (Variables|Default|SetcanOpenDoor false)
  (bind _asbp_first_person_character (Utilities|Casting|CastToBP_FirstPersonCharacter OtherActor))
  (Widget|SetVisibility (stale OnComponentBeginOverlap(Collider) _returnvalue) "Hidden")
  (Variables|/Game/FirstPerson/Blueprints/BP_FirstPersonCharacter.BP_FirstPersonCharacter_C|SetDoor _asbp_first_person_character 0))

(event Custom|Open%20Door
  (bind _asgm_save_load (Utilities|Casting|CastToGM_SaveLoad (Game|GetGameMode)))
  (Default|AddActors (Variables|/Game/Blueprints/SaveLoad/GM_SaveLoad.GM_SaveLoad_C|GetLevelState _asgm_save_load) self)
  (CallFunction|OpenDoor))

(event EventBeginPlay)

(event Collision|EventActorBeginOverlap
  (params (OtherActor :type Actor%20Object%20Reference)))

(event EventTick
  (params (DeltaSeconds :type Float%20%28single-precision%29)))

(event EventActivate
  (CallFunction|OpenDoor))

(fn ConstructionScript
  (Transformation|AddLocalRotation (Variables|Default|GetSM_Door_03) (Math|Rotator|MakeRotator 0.0 0.0 (Variables|Door|GetDoor%20Rotation)) false false))

(fn OpenDoor
  (Class|Actor|AddActorWorldRotation "0.000000,90.000000,0.000000"))